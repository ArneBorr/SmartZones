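; Smart zone Blueprint that configures its roles and triggers from an XML script loaded on BeginPlay.
; Role entries become structs (name, single-digit min/max cardinality, dynamic-join flag) registered with MPRoleManager.
; Triggers, read only when roles are found, are constructed as objects in MPTriggerManager.
; Each trigger receives indexed conditions by name, using the ConditionRepo on the player's FirstPersonCharacter.
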(event `self.ReceiveBeginPlay`
  ;[1 1 1] GetScript
  (bind (_errormessage _returnvalue) (`EasyXMLParseManager.LoadFromFile` (`KismetStringLibrary.Concat_StrStr` (`self.FilePath`) (`self.ScriptName`) ".xml"))
    (:`Successed`
      (bind _returnvalue_2 (`EasyXMLElement.ReadElements` _returnvalue "SmartZone.Role")
        (:`Found`
          (for _array_element _returnvalue_2
            (bind _role (`self.ReadRole` _array_element))
            (`RoleManager.AddRole` (`self.m_pRoleManager`) _role))
          (bind _returnvalue_3 (`EasyXMLElement.ReadElements` _returnvalue "SmartZone.Trigger")
            (:`Found`
              (for _array_element_2 _returnvalue_3
                (`self.Handle New Trigger` _array_element_2)))))))))

(fn `Handle New Trigger`
  (params (TriggerXML :type "EasyXMLElement Object Reference"))
  (bind _m_ptriggermanager (`self.m_pTriggerManager`))
  (bind _asfirst_person_character (cast `/Game/FirstPersonCPP/Blueprints/FirstPersonCharacter` (`GameplayStatics.GetPlayerCharacter` 0)))
  (bind _returnvalue (`|GenericCreateObject` "/Script/GW_SmartZones.Trigger" _m_ptriggermanager))
  (`TriggerManager.AddTrigger` _m_ptriggermanager _returnvalue)
  (bind _result (`/Engine/EditorBlueprintResources/StandardMacros.DecrementInt` (`KismetStringLibrary.Conv_StringToInt` (`EasyXMLElement.ReadString` TriggerXML "NrOfConditions" "")))
    (:`  `
      (for _index (range (+ _result 1))
        (bind _returnvalue_2 (`EasyXMLElement.ReadElement` TriggerXML (`KismetStringLibrary.Concat_StrStr` (`self.Access String`) (`KismetStringLibrary.Conv_IntToString` _index)))
          (:`Found`
            (`Trigger.AddCondition` _returnvalue (`/Game/FirstPersonCPP/Blueprints/FirstPersonCharacter.Condition Repo` _asfirst_person_character) (`EasyXMLObject.GetStringValue` _returnvalue_2 ""))))))))

(fn `ReadRole`
  (params (RoleXML :type "EasyXMLElement Object Reference"))
  (returns (Role :type "Role Structure"))
  (bind _returnvalue (`EasyXMLElement.ReadString` RoleXML "Name" ""))
  (bind _returnvalue_2 (`EasyXMLElement.ReadString` RoleXML "Cardinality" ""))
  (`KismetSystemLibrary.PrintString` _returnvalue)
  (return (make `Role` _returnvalue (`KismetStringLibrary.Conv_StringToInt` (`KismetStringLibrary.GetSubstring` _returnvalue_2)) (`KismetStringLibrary.Conv_StringToInt` (`KismetStringLibrary.GetSubstring` _returnvalue_2 2)) 0 (`KismetMathLibrary.Conv_IntToBool` (`KismetStringLibrary.Conv_StringToInt` (`EasyXMLElement.ReadString` RoleXML "Flags.CanJoinDynamically" ""))))))

(fn `UserConstructionScript`)